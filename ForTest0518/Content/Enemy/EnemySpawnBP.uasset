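; Enemy spawner actor that periodically fills a box volume with EnemyBP AI pawns while the enemy count is within a fixed cap.
; On BeginPlay it caches the ShooterGameMode and starts a looping half-second timer on SpawnEnemy.
; Each tick of that timer checks the game mode's NumberEnemies, spawns at a random point inside SpawningBox, then increments the shared count.
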(event `self.ReceiveBeginPlay`
  (bind _asshooter_game_mode (cast `/Game/ShooterGameMode` (`GameplayStatics.GetGameMode`)))
  (set `self.GameMode` _asshooter_game_mode)
  (`KismetSystemLibrary.K2_SetTimer` null "SpawnEnemy" 0.5 true))

(event `SpawnEnemy`
  (bind _spawning_box (`self.Spawning box`))
  (bind _gamemode (`self.GameMode`))
  (if (<= (`/Game/ShooterGameMode.NumberEnemies` _gamemode) 10)
    (`AIBlueprintHelperLibrary.SpawnAIFromClass` "/Game/Enemy/EnemyBP.EnemyBP_C" null (`KismetMathLibrary.RandomPointInBoundingBox` (`SceneComponent.K2_GetComponentLocation` _spawning_box) (`BoxComponent.GetScaledBoxExtent` _spawning_box)))
    (`/Game/ShooterGameMode.IncreaseNumberEnemies` _gamemode)))

(fn `UserConstructionScript`)